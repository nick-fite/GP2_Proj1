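; Test character Blueprint for trying fighting-game input combos, with crouch and a double jump.
; BeginPlay registers two directional-plus-attack sequences on FightingInput with event callbacks, alongside punch and death montage functions.
; Jump launches the character through a DoN limited to two uses, reset on landing.
; An unconnected graph holds an older-style combo check that steps through buffered inputs using a frame-based delay macro.
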(event `EnhancedInput|/Game/_MyFiles/Inputs/IA_Jump`
  (params (ActionValue :type Boolean) (ElapsedSeconds :type "Float (double-precision)") (TriggeredSeconds :type "Float (double-precision)") (InputAction :type "InputAction Object Reference" :default "/Game/_MyFiles/Inputs/IA_Jump.IA_Jump"))
  (:`Started`
    (`/Engine/EditorBlueprintResources/StandardMacros.Do N` 2 :!label _label
      (:`Exit`
        (`self.LaunchCharacter` (`KismetMathLibrary.MakeVector` 0.0 0.0 (`CharacterMovementComponent.JumpZVelocity` (`self.CharacterMovement`))) false true)))))

(event `EnhancedInput|/Game/_MyFiles/Inputs/IA_Crouch`
  (params (ActionValue :type Boolean) (ElapsedSeconds :type "Float (double-precision)") (TriggeredSeconds :type "Float (double-precision)") (InputAction :type "InputAction Object Reference" :default "/Game/_MyFiles/Inputs/IA_Crouch.IA_Crouch"))
  (:`Triggered`
    (`self.Crouch`))
  (:`Completed`
    (`self.UnCrouch`)))

(event `self.OnLanded`
  (params (Hit :type "HitResult Structure (by ref)"))
  (goto _label :!via `Reset`))

(event `EnhancedInput|/Game/_MyFiles/Inputs/IA_FightingInputDown`
  (params (ActionValue :type Boolean) (ElapsedSeconds :type "Float (double-precision)") (TriggeredSeconds :type "Float (double-precision)") (InputAction :type "InputAction Object Reference" :default "/Game/_MyFiles/Inputs/IA_FightingInputDown.IA_FightingInputDown")))

(event `self.ReceiveBeginPlay`
  (bind _fightinginput (`self.FightingInput`))
  (`InputSystem.AddCombo` _fightinginput (`|MakeArray` "Up" "Up" "Normal" :!type "EInputType Enum") (`|CreateDelegate` :!event `DeathAnim`))
  (`InputSystem.AddCombo` _fightinginput (`|MakeArray` "Right" "Left" "Special" :!type "EInputType Enum") (`|CreateDelegate` :!event `PunchAnim`)))

(fn `DeathAnim`
  (`self.PlayAnimMontage` "/Game/_MyFiles/Anim/DeathAnimUsable_Montage.DeathAnimUsable_Montage"))

(fn `PunchAnim`
  (`self.PlayAnimMontage` "/Game/_MyFiles/Anim/Hook_PunchUE5_Montage.Hook_PunchUE5_Montage"))

(fn `UserConstructionScript`)